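; BP_projectile_zombie is a projectile that turns defeated enemies into zombies.
; On hit it applies a radial impulse with strain to the struck component, then destroys itself.
; If the hit actor is an injured BazaEnemy with no health left, it sets that enemy's transform flag, calls Transform and prints a debug message.
; Tick destroys the projectile once it reaches MaxDistance from its spawn location.
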(event EventHit
  (params (MyComp :type Primitive%20Component%20Object%20Reference) (Other :type Actor%20Object%20Reference) (OtherComp :type Primitive%20Component%20Object%20Reference) (bSelfMoved :type Boolean) (HitLocation :type Vector :default "0, 0, 0") (HitNormal :type Vector :default "0, 0, 0") (NormalImpulse :type Vector :default "0, 0, 0") (Hit :type Hit%20Result%20Structure%20%28by%20ref%29))
  (Class|PhysicsObjectBlueprintLibrary|ApplyRadialImpulse OtherComp HitLocation 2e+02 2e+03 "RIF_Constant" true 6e+05 false 0.0 1.0)
  (bind _asbaza_enemy (Utilities|Casting|CastToBazaEnemy (.HitActor (Collision|BreakHitResult Hit)))
    (:then
      (if (and (Variables|/Game/AI/itsbaza/BazaEnemy.BazaEnemy_C|Getisinjured _asbaza_enemy) (<= (Variables|/Game/AI/itsbaza/BazaEnemy.BazaEnemy_C|GetHealth _asbaza_enemy) 0))
        (Variables|/Game/AI/itsbaza/BazaEnemy.BazaEnemy_C|Settransformb _asbaza_enemy true)
        (Default|Transform _asbaza_enemy)
        (Development|PrintString "Yoe are zombie ")))
    (:CastFailed
      _))
  (Actor|DestroyActor))

(event EventBeginPlay
  (Variables|Default|Setspawn%20loc (Transformation|GetActorLocation)))

(event EventTick
  (params (DeltaSeconds :type Float%20%28single-precision%29))
  (if (>= (Math|Vector|Distance(Vector) (Transformation|GetActorLocation) (Variables|Default|Getspawn%20loc)) (Variables|Default|Getmax%20distance))
    (Actor|DestroyActor)))

(fn ConstructionScript
  (|CallParentFunction))