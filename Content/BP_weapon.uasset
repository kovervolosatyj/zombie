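; BP_weapon is a weapon actor that fires BP_projectile_simple projectiles from a limited ammo count.
; Shoot spawns a projectile at the weapon's transform with the player character as instigator and decrements ammo; when empty, it calls StopShooting and Reload.
; Reload waits for a delay, then refills to maximum, with debug prints marking progress.
; StartShooting and StopShooting are empty events, and an actor-attach node is left unconnected.
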(event Custom|reload
  ;[0.15 0.15 0.15 0.5] перезарядка
  (Development|PrintString "start reloading")
  (Utilities|FlowControl|Delay (Variables|Default|GetDuration))
  (Variables|Default|Setcurrent%20ammos (Variables|Default|Getmax%20ammos))
  (Development|PrintString "reloading finished"))

(event Custom|shoot
  (if (> (Variables|Default|Getcurrent%20ammos) 0)
    (Game|SpawnActorfromClass "/Game/BP_projectile_simple.BP_projectile_simple_C" (Transformation|GetActorTransform) "Undefined" "MultiplyWithRoot" 0 (Game|GetPlayerCharacter 0))
    (Math|Integer|DecrementInt (Variables|Default|Getcurrent%20ammos))
    (else
      (CallFunction|StopShooting)
      (Development|PrintString "no ammo")
      (CallFunction|Reload))))

(event Custom|start%20shooting)

(event Custom|stop%20shooting)

(fn ConstructionScript)