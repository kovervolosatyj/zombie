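; BP_weapon_automathic is an automatic weapon Blueprint that controls repeat fire with a looping timer.
; StartShooting starts a short-interval looping timer bound to an event and stores its handle in ShootingTimer.
; StopShooting clears and invalidates that handle to end the loop.
; The per-shot logic is not visible in this graph, and BeginPlay, overlap and Tick are disabled stubs.
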(event EventBeginPlay
  (|CallParentFunction) ; This node is disabled and will not be called.\nDrag off pins to build functionality.
)

(event Collision|EventActorBeginOverlap
  (params (OtherActor :type Actor%20Object%20Reference))
  (|CallParentFunction OtherActor) ; This node is disabled and will not be called.\nDrag off pins to build functionality.
)

(event EventTick
  (params (DeltaSeconds :type Float%20%28single-precision%29))
  (|CallParentFunction DeltaSeconds) ; This node is disabled and will not be called.\nDrag off pins to build functionality.
)

(event EventStartShooting
  (bind _returnvalue (Utilities|Time|SetTimerbyEvent (EventDispatchers|CreateEvent :!event Shoot) 0.2 true))
  (Variables|Default|Setshooting%20timer _returnvalue))

(event EventStopShooting
  (Utilities|Time|ClearandInvalidateTimerbyHandle (Variables|Default|Getshooting%20timer)))

(fn ConstructionScript
  (|CallParentFunction))