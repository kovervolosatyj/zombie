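; Tutorial AI character that becomes injured at zero health and can transform into a zombie.
; Damage handlers clamp health, then flag injury and start a delayed timer, while BeginPlay sets health to zero.
; Transform swaps mesh materials, tells the BazaEnemyCtrl AI controller to transform and hides the widget.
; A widget event sequences tutorial actors BP_tutor1 and BP_tutor5, but its low-health trigger is disconnected.
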(event Custom|widgets
  (bind _asbp_tutor_1 (Utilities|Casting|CastToBP_tutor1 (Variables|Default|Getwi1)))
  (Default|Widgetendless _asbp_tutor_1)
  (Actor|DestroyActor _asbp_tutor_1)
  (Utilities|FlowControl|Delay 0.8)
  (Rendering|SetVisibility (Variables|Default|GetWidget) true false)
  (Utilities|FlowControl|Delay 1.0)
  (bind _asbp_tutor_5 (Utilities|Casting|CastToBP_tutor5 (Variables|Default|Getwi2)))
  (Default|Begin _asbp_tutor_5))

(event Custom|CustomEvent
  (if (Variables|Default|Gettransformb)
    (CallFunction|Transform)))

(event Custom|CustomEvent_1
  (params (Damage :type Float%20%28single-precision%29) (DamageType :type Damage%20Type%20Object%20Reference) (InstigatedBy :type Controller%20Object%20Reference) (DamageCauser :type Actor%20Object%20Reference))
  ;[0.15 0.15 0.15 0.5] дамаг и превращение
  (Variables|Default|SetHealth (Math|Float|Clamp(Float) (- (Variables|Default|GetHealth) Damage) 0.0 (Variables|Default|Getmax%20heath)))
  (if (<= (Variables|Default|GetHealth) 0.0)
    (Variables|Default|Setisinjured true)
    (Utilities|Time|SetTimerbyEvent (EventDispatchers|CreateEvent :!event Expired) 3.0)
    (else
      (Development|PrintString (Utilities|String|ToString(Float) (Variables|Default|GetHealth)) true true "(R=1.000000,G=0.007400,B=0.501092,A=1.000000)"))))

(event EventBeginPlay
  (|CallParentFunction)
  (Variables|Default|SetHealth 0.0))

(event Collision|EventActorBeginOverlap
  (params (OtherActor :type Actor%20Object%20Reference))
  ;[0.15 0.15 0.15 0.5] дамаг и превращение
  (|CallParentFunction OtherActor) ; This node is disabled and will not be called.\nDrag off pins to build functionality.
)

(event EventTick
  (params (DeltaSeconds :type Float%20%28single-precision%29))
  (|CallParentFunction DeltaSeconds))

(event Game|Damage|EventAnyDamage
  (params (Damage :type Float%20%28single-precision%29) (DamageType :type Damage%20Type%20Object%20Reference) (InstigatedBy :type Controller%20Object%20Reference) (DamageCauser :type Actor%20Object%20Reference))
  ;[0.15 0.15 0.15 0.5] дамаг и превращение
  (Variables|Default|SetHealth (Math|Float|Clamp(Float) (- (Variables|Default|GetHealth) Damage) 0.0 (Variables|Default|Getmax%20heath)))
  (if (<= (Variables|Default|GetHealth) 0.0)
    (Variables|Default|Setisinjured true)
    (Utilities|Time|SetTimerbyEvent (EventDispatchers|CreateEvent :!event Expired) 3.0)
    (else
      (Development|PrintString (Utilities|String|ToString(Float) (Variables|Default|GetHealth)) true true "(R=1.000000,G=0.007400,B=0.501092,A=1.000000)"))))

(event EventTransform
  (bind _mesh (Variables|Character|GetMesh))
  (if (Variables|Default|Getisinjured)
    (Rendering|Material|SetMaterial _mesh 0 "/Game/M_zombie_color.M_zombie_color")
    (Rendering|Material|SetMaterial _mesh 1 "/Game/M_zombie_color.M_zombie_color")
    (Variables|Default|Setiszombie true)
    (bind _asbaza_enemy_ctrl (Utilities|Casting|CastToBazaEnemyCtrl (AI|GetAIController self)))
    (Variables|/Game/AI/itsbaza/BazaEnemyCtrl.BazaEnemyCtrl_C|SetIszombie _asbaza_enemy_ctrl true)
    (Default|TRANSFORM _asbaza_enemy_ctrl)
    (Rendering|SetVisibility (Variables|Default|GetWidget) false false)))

(fn ConstructionScript
  (|CallParentFunction))