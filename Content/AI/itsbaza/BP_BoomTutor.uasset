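; Tutorial enemy Blueprint that advances the tutorial widget sequence when its health runs low.
; BeginPlay runs parent setup and calls Appear; Tick fires the widgets event once when Health drops below 30, gated by a bool.
; That event ends and destroys the BP_tutor1 actor, shows Widget0, then starts BP_tutor5, with short delays between.
; The Transform event is empty, and leftover zombie-conversion and camera-facing logic is disconnected.
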(event Custom|widgets
  (bind _asbp_tutor_1 (Utilities|Casting|CastToBP_tutor1 (Variables|Default|Getwi1)))
  (Default|Widgetendless _asbp_tutor_1)
  (Actor|DestroyActor _asbp_tutor_1)
  (Utilities|FlowControl|Delay 0.8)
  (Rendering|SetVisibility (Variables|Default|GetWidget_0) true false)
  (Utilities|FlowControl|Delay 1.0)
  (bind _asbp_tutor_5 (Utilities|Casting|CastToBP_tutor5 (Variables|Default|Getwi2)))
  (Default|Begin _asbp_tutor_5))

(event EventBeginPlay
  (|CallParentFunction)
  (CallFunction|Appear))

(event Collision|EventActorBeginOverlap
  (params (OtherActor :type Actor%20Object%20Reference)))

(event EventTick
  (params (DeltaSeconds :type Float%20%28single-precision%29))
  (|CallParentFunction DeltaSeconds)
  (if (and (Variables|Default|GetIf) (< (Variables|Default|GetHealth) 3e+01))
    (CallFunction|Widgets)
    (Variables|Default|SetIf false)))

(event EventTransform)

(fn ConstructionScript
  (|CallParentFunction))