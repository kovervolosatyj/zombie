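; BP_Shiza is an AI character that knocks the player's weapon away on contact.
; On overlap, if its Health is 50 or less and Iszombie is false, it replaces the player's current weapon with its pickup actor and briefly shows a "stolen" widget.
; Custom events drive ABP_Zombie1: one clears Sleep, the other pulses Angry at low health.
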(event Custom|ABP
  (bind _asabp_zombie_1 (Utilities|Casting|CastToABP_Zombie1 (Components|SkeletalMesh|GetAnimInstance (Variables|Character|GetMesh))))
  (Variables|/Game/AI/ZombieMesh/ABP_Zombie1.ABP_Zombie1_C|Setsleep _asabp_zombie_1 false))

(event Custom|angruABP
  (if (< (Variables|Default|GetHealth) 5e+01)
    (bind _asabp_zombie_1 (Utilities|Casting|CastToABP_Zombie1 (Components|SkeletalMesh|GetAnimInstance (Variables|Character|GetMesh))))
    (Variables|/Game/AI/ZombieMesh/ABP_Zombie1.ABP_Zombie1_C|Setangry _asabp_zombie_1 true)
    (Utilities|FlowControl|Delay 0.5)
    (Variables|/Game/AI/ZombieMesh/ABP_Zombie1.ABP_Zombie1_C|Setangry _asabp_zombie_1 false)
    (else
      (Variables|/Game/AI/ZombieMesh/ABP_Zombie1.ABP_Zombie1_C|Setangry _asabp_zombie_1 false))))

(event Collision|EventActorBeginOverlap
  (params (OtherActor :type Actor%20Object%20Reference))
  (|CallParentFunction OtherActor)
  (if (not (> (Variables|Default|GetHealth) 50))
    (if (not (Variables|Default|Getiszombie))
      (bind _asbp_first_person_character (Utilities|Casting|CastToBP_FirstPersonCharacter OtherActor))
      (bind _current_weapon (Variables|/Game/FirstPerson/Blueprints/BP_FirstPersonCharacter.BP_FirstPersonCharacter_C|Getcurrent%20weapon _asbp_first_person_character)
        (:then
          (Variables|Default|SetCurrent%20Weapon _current_weapon)
          (Game|SpawnActorfromClass (Variables|/Game/Weapons/BP_weapon.BP_weapon_C|Getweapon_pick_up (Variables|Default|GetCurrent%20Weapon)) (Transformation|GetActorTransform (Variables|Default|GetCurrent%20Weapon)) "Undefined" "MultiplyWithRoot" 0 0)
          (Actor|DestroyActor _current_weapon)
          (bind _returnvalue (UserInterface|CreateWidget "/Game/widgets/WB_stolen.WB_stolen_C"))
          (UserInterface|Viewport|AddtoViewport _returnvalue 0)
          (Utilities|FlowControl|Delay 1.0)
          (Widget|RemovefromParent _returnvalue))
        (:else)))))

(fn ConstructionScript
  (|CallParentFunction))