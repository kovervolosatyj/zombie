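; Shotgun weapon Blueprint that fires a ten-projectile spread from the player's camera direction for each round of ammo.
; StartShooting spends one round and spawns the configured projectile class at the shoot arrow, using SprayRadius to randomize offset and direction.
; Auto projectiles receive the weapon's damage and range unless they are zombie variants, and each triggers a camera shake.
; An empty magazine stops shooting and reloads.
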(event Custom|simple%20shake
  (bind _asbp_first_person_character (Utilities|Casting|CastToBP_FirstPersonCharacter (Game|GetPlayerCharacter 0)))
  (Default|CameraShake _asbp_first_person_character))

(event EventStartShooting
  (bind _returnvalue (Game|GetPlayerCharacter 0))
  ;[0.15 0.15 0.15 0.5] обычные пули
  (bind _asbp_first_person_character (Utilities|Casting|CastToBP_FirstPersonCharacter _returnvalue))
  (if (> (Variables|Default|Getcurrent%20ammos) 0)
    (bind _result (Math|Integer|DecrementInt (Variables|Default|Getcurrent%20ammos))
      (:%20%20
        (Development|PrintString (Utilities|String|ToString(Integer) _result))
        (for _index (range 1 10)
          (bind _returnvalue_2 (Game|SpawnActorfromClass (Variables|Default|GetClass_0) (Math|Transform|MakeTransform (+ (Transformation|GetWorldLocation (Variables|Default|Getshoot%20arrow)) (CallFunction|SprayRadius (Math|Vector|GetForwardVector (Transformation|GetWorldRotation (Variables|/Game/FirstPerson/Blueprints/BP_FirstPersonCharacter.BP_FirstPersonCharacter_C|GetFirstPersonCamera _asbp_first_person_character))) (Variables|Default|GetMax%20Angle))) (CallFunction|SprayRadius (Math|Vector|GetForwardVector (Transformation|GetWorldRotation (Variables|/Game/FirstPerson/Blueprints/BP_FirstPersonCharacter.BP_FirstPersonCharacter_C|GetFirstPersonCamera _asbp_first_person_character))) (Variables|Default|GetMax%20Angle))) "AlwaysSpawn" "MultiplyWithRoot" 0 _returnvalue))
          (bind _asbp_projectile_auto (Utilities|Casting|CastToBP_projectile_auto _returnvalue_2))
          (if (Utilities|ClassIsChildOf (Utilities|GetClass _asbp_projectile_auto) "/Game/bullets/BP_projectile_zombi.BP_projectile_zombi_C")
            (CallFunction|SimpleShake)
            (else
              (Variables|/Game/bullets/BP_projectile_auto.BP_projectile_auto_C|SetBase%20Damage _asbp_projectile_auto (Variables|Default|Getbullet%20damage))
              (Development|PrintString "Hello")
              (Variables|/Game/bullets/BP_projectile_auto.BP_projectile_auto_C|Setmax%20distance _asbp_projectile_auto (Variables|Default|GetMax%20Distance))
              (CallFunction|SimpleShake))))))
    (else
      (CallFunction|StopShooting)
      (Development|PrintString "no ammo")
      (CallFunction|Reload))))

(fn ConstructionScript
  (|CallParentFunction))