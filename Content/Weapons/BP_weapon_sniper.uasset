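; Sniper weapon Blueprint with a charge-up shot, built on parent weapon logic.
; StartShooting plays a timeline that drives Currentcharge, firing and triggering the first-person character's sniper camera shake at full charge.
; StopShooting also fires, shakes and stops the timeline, but only above a minimum charge and when IsShooting is clear.
; IsHolding and IsShooting gate both events; neither event resets IsHolding.
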(event Custom|sniper%20shake
  (bind _asbp_first_person_character (Utilities|Casting|CastToBP_FirstPersonCharacter (Game|GetPlayerCharacter 0)))
  (Default|CameraShakeSniper _asbp_first_person_character))

(event EventStartShooting
  (if (and (not (Variables|Default|Getis%20holding)) (<= (Variables|Default|Getcurrentcharge) 0.2))
    (if (not (Variables|Default|Getis_shooting))
      (Variables|Default|Setis_shooting true)
      (Variables|Default|Setis%20holding true)
      (bind _charging (Timeline|Timeline Play)
        (:Update
          (bind _output_get (Variables|Default|Setcurrentcharge (Math|Float|Clamp(Float) _charging)))
          (if (>= _output_get 1.0)
            (CallFunction|Shoot)
            (CallFunction|SniperShake)
            (Variables|Default|Setis_shooting false)))))))

(event EventStopShooting
  (if (and (Variables|Default|Getis%20holding) (>= (Variables|Default|Getcurrentcharge) 0.2))
    (if (not (Variables|Default|Getis_shooting))
      (Variables|Default|Setis_shooting true)
      (CallFunction|Shoot)
      (CallFunction|SniperShake)
      (Variables|Default|Setis_shooting false)
      (bind _charging (Timeline|Timeline Stop)
        (:Update
          (bind _output_get (Variables|Default|Setcurrentcharge (Math|Float|Clamp(Float) _charging)))
          (if (>= _output_get 1.0)
            (CallFunction|Shoot)
            (CallFunction|SniperShake)
            (Variables|Default|Setis_shooting false)))))))

(fn ConstructionScript
  (|CallParentFunction))