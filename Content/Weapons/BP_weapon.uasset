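; Weapon Blueprint for the first-person character that fires switchable base or zombie projectiles and handles ammo and reloading.
; Shoot spawns the selected class near ShootArrow along camera rotation, applying bullet damage and spending ammo only for non-zombie BP_projectile_auto rounds.
; An empty magazine triggers Reload, which plays character and weapon montages, then refills after a delay.
; Start/stop and zombie-shoot events are empty; a cone-spread helper exists but is not called here.
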(event Custom|reload
  (Variables|Default|Setcab%20shoot false)
  (Utilities|FlowControl|Sequence
    (:then_0
      (bind _asbp_first_person_character (Utilities|Casting|CastToBP_FirstPersonCharacter (Game|GetPlayerCharacter 0)))
      (Animation|Montage|PlayMontage (Variables|/Game/FirstPerson/Blueprints/BP_FirstPersonCharacter.BP_FirstPersonCharacter_C|GetFirstPersonMesh _asbp_first_person_character) (Variables|Default|GetMontage%20to%20Play_1) 1.0 0.0 "None" false))
    (:then_1
      (Animation|Montage|PlayMontage (Variables|Default|Getpistol) (Variables|Default|GetMontage%20to%20Play_2) 1.0 0.0 "None" false))
    (:then_2
      (Development|PrintString "start reloading")
      (Variables|Default|Setcurrent%20ammos 0)
      (Utilities|FlowControl|Delay (Variables|Default|GetDuration))
      (Variables|Default|Setcurrent%20ammos (Variables|Default|Getmax%20ammos))
      (Development|PrintString "reloading finished")
      (Variables|Default|Setcab%20shoot true))))

(event Custom|switchZ
  (Variables|Default|SetClass_0 (Variables|Default|Getzombie_bullet)))

(event Custom|switchB
  (Variables|Default|SetClass_0 (Variables|Default|Getbase%20bullet)))

(event Custom|Zombie%20shoot)

(event Custom|Shoot
  (bind _returnvalue (Game|GetPlayerCharacter 0))
  ;[0.15 0.15 0.15 0.5] обычные пули
  (bind _asbp_first_person_character (Utilities|Casting|CastToBP_FirstPersonCharacter _returnvalue))
  (if (> (Variables|Default|Getcurrent%20ammos) 0)
    (bind _returnvalue_2 (Game|SpawnActorfromClass (Variables|Default|GetClass_0) (Math|Transform|MakeTransform (+ (Transformation|GetWorldLocation (Variables|Default|Getshoot%20arrow)) (Transformation|GetWorldRotation (Variables|/Game/FirstPerson/Blueprints/BP_FirstPersonCharacter.BP_FirstPersonCharacter_C|GetFirstPersonCamera _asbp_first_person_character))) (Transformation|GetWorldRotation (Variables|/Game/FirstPerson/Blueprints/BP_FirstPersonCharacter.BP_FirstPersonCharacter_C|GetFirstPersonCamera _asbp_first_person_character))) "AlwaysSpawn" "MultiplyWithRoot" _returnvalue 0))
    (bind _asbp_projectile_auto (Utilities|Casting|CastToBP_projectile_auto _returnvalue_2))
    (if (not (Utilities|ClassIsChildOf (Utilities|GetClass _asbp_projectile_auto) "/Game/bullets/BP_projectile_zombi.BP_projectile_zombi_C"))
      (Variables|/Game/bullets/BP_projectile_auto.BP_projectile_auto_C|SetBase%20Damage _asbp_projectile_auto (Variables|Default|Getbullet%20damage))
      (bind _result (Math|Integer|DecrementInt (Variables|Default|Getcurrent%20ammos))
        (:%20%20
          (Development|PrintString (Utilities|String|ToString(Integer) _result)))))
    (else
      (CallFunction|StopShooting)
      (Development|PrintString "no ammo")
      (if (Variables|Default|Getcab%20shoot)
        (CallFunction|Reload)))))

(event Custom|stop%20shooting)

(event Custom|stop%20zombie%20shoot)

(event Custom|start%20shooting)

(fn ConstructionScript)

(fn SprayRadius
  (params (muzzle%20d :type Vector) (max%20angle :type Float%20%28double-precision%29))
  (return (Math|Conversions|RotationFromXVector (Math|Random|RandomUnitVectorinConeinDegrees muzzle%20d max%20angle))))

(fn Switchammos)