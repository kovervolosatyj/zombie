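; Automatic weapon Blueprint that provides sustained fire with camera shake while shooting is active.
; StartShooting calls Shoot and AutoShaking immediately, then starts two looping timers stored as ShootingTimer and ShakeTimer.
; AutoShaking casts the player character to BP_FirstPersonCharacter and triggers its CameraShakeAuto.
; StopShooting clears both timers to end the repeating cycle.
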(event Custom|auto%20shaking
  (bind _asbp_first_person_character (Utilities|Casting|CastToBP_FirstPersonCharacter (Game|GetPlayerCharacter 0)))
  (Default|CameraShakeAuto _asbp_first_person_character))

(event EventStartShooting
  (Utilities|FlowControl|Sequence
    (:then_0
      (CallFunction|Shoot)
      (CallFunction|AutoShaking))
    (:then_1
      (bind _returnvalue (Utilities|Time|SetTimerbyEvent (EventDispatchers|CreateEvent :!event Shoot) 0.2 true))
      (Variables|Default|Setshooting%20timer _returnvalue)
      (bind _returnvalue_2 (Utilities|Time|SetTimerbyEvent (EventDispatchers|CreateEvent :!event Custom|auto%20shaking) 0.2 true))
      (Variables|Default|Setshake%20timer _returnvalue_2))))

(event EventStopShooting
  (Utilities|Time|ClearandInvalidateTimerbyHandle (Variables|Default|Getshooting%20timer))
  (Utilities|Time|ClearandInvalidateTimerbyHandle (Variables|Default|Getshake%20timer)))

(fn ConstructionScript
  (|CallParentFunction))