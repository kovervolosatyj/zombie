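; Automatic-weapon projectile, judging by its name, that deals damage on impact and destroys itself on hit or after exceeding a max travel distance from spawn.
; On hit it attaches a short-lived bullet-hole decal and applies a radial impulse with strain to the struck component.
; BazaEnemy targets get a Niagara effect and damage.
; Hits also trigger BP_ButtonWall's Do and BP_Shiza's AngruABP.
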(event Collision|EventHit
  (params (MyComp :type Primitive%20Component%20Object%20Reference) (Other :type Actor%20Object%20Reference) (OtherComp :type Primitive%20Component%20Object%20Reference) (bSelfMoved :type Boolean) (HitLocation :type Vector :default "0, 0, 0") (HitNormal :type Vector :default "0, 0, 0") (NormalImpulse :type Vector :default "0, 0, 0") (Hit :type Hit%20Result%20Structure%20%28by%20ref%29))
  (bind (_bblockinghit _binitialoverlap _time _distance _location _impactpoint _normal _impactnormal _physmat _hitactor) (Collision|BreakHitResult Hit))
  (Utilities|FlowControl|Sequence
    (:then_0
      (Class|GameplayStatics|SpawnDecalAttached "/Game/decal/M_bullet_hole.M_bullet_hole" "6.500000,13.000000,13.000000" OtherComp "None" HitLocation (Math|Conversions|RotationFromXVector HitNormal) "KeepWorldPosition" 5.0)
      (Class|PhysicsObjectBlueprintLibrary|ApplyRadialImpulse OtherComp HitLocation 2e+02 2e+03 "RIF_Constant" true (Variables|Default|GetStrain) false 0.0 1.0)
      (bind _asbaza_enemy (Utilities|Casting|CastToBazaEnemy _hitactor)
        (:then
          (Niagara|SpawnSystematLocation "/Game/niagara/NS_damage_bb.NS_damage_bb" _location)
          (Game|Damage|ApplyDamage _asbaza_enemy (Variables|Default|GetBase%20Damage) 0 0))
        (:CastFailed
          _))
      (Actor|DestroyActor))
    (:then_1
      (bind _asbp_button_wall (Utilities|Casting|CastToBP_ButtonWall _hitactor))
      (Default|Do _asbp_button_wall))
    (:then_2
      (bind _asbp_shiza (Utilities|Casting|CastToBP_Shiza _hitactor))
      (Default|AngruABP _asbp_shiza))))

(event EventBeginPlay
  (Variables|Default|Setspawn%20loc (Transformation|GetActorLocation)))

(event EventTick
  (params (DeltaSeconds :type Float%20%28single-precision%29))
  (if (>= (Math|Vector|Distance(Vector) (Transformation|GetActorLocation) (Variables|Default|Getspawn%20loc)) (Variables|Default|Getmax%20distance))
    (Actor|DestroyActor)))

(fn ConstructionScript)