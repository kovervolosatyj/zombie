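; Sniper rifle pickup that equips the interacting player character with a sniper weapon.
; On Interact, it destroys the character's current weapon if it differs from their Sniper reference, then spawns BP_weapon_sniper at the pickup's transform and destroys itself.
; The new weapon becomes CurrentWeapon and snaps to the weapon_socket on the first-person mesh, with a debug print of its name.
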(event EventInteract
  (params (player%20character :type BP%20First%20Person%20Character%20Object%20Reference))
  (bind _sniper (Variables|/Game/FirstPerson/Blueprints/BP_FirstPersonCharacter.BP_FirstPersonCharacter_C|Getsniper player%20character))
  (if (!= (stale _output_get) _sniper)
    (Utilities|IsValid (stale _output_get_2)
      (:Is%20Valid
        (Actor|DestroyActor (stale _output_get)))
      (:Is%20Not%20Valid
        _)))
  (bind _output_get (Variables|/Game/FirstPerson/Blueprints/BP_FirstPersonCharacter.BP_FirstPersonCharacter_C|Setcurrent%20weapon player%20character _sniper))
  ;[0.15 0.15 0.15 0.5] спавн
  (bind _returnvalue (Game|SpawnActorfromClass "/Game/Weapons/BP_weapon_sniper.BP_weapon_sniper_C" (Transformation|GetActorTransform) "AlwaysSpawn" "MultiplyWithRoot" 0 0))
  ;[0.15 0.15 0.15 0.5] уничтожение модельки на земле
  (Actor|DestroyActor)
  (Development|PrintString (Utilities|GetDisplayName _returnvalue))
  ;[0.15 0.15 0.15 0.5] присоединяем к сокету
  (bind _output_get_2 (Variables|/Game/FirstPerson/Blueprints/BP_FirstPersonCharacter.BP_FirstPersonCharacter_C|Setcurrent%20weapon player%20character _returnvalue))
  (Transformation|AttachComponentToComponent _output_get_2 (Variables|/Game/FirstPerson/Blueprints/BP_FirstPersonCharacter.BP_FirstPersonCharacter_C|GetFirstPersonMesh player%20character) "weapon_socket" "SnapToTarget" "SnapToTarget" "SnapToTarget" true))

(fn ConstructionScript
  (|CallParentFunction))